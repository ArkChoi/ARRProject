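; Robot arm actor that constrains the rotation of three sphere components, likely serving as its joints.
; Every Tick runs the SphereLimited helper on the first, second and third spheres.
; The helper rewrites each sphere's world rotation, keeping pitch clamped within a quarter turn either way and forcing roll and yaw to zero.
; The limit applies in world space, independent of any parent rotation.
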(event EventTick
  (params (DeltaSeconds :type Float%20%28single-precision%29))
  (CallFunction|SphereLimited (Variables|Default|GetFirstSphere))
  (CallFunction|SphereLimited (Variables|Default|GetSecondSphere))
  (CallFunction|SphereLimited (Variables|Default|GetThridSphere)))

(fn ConstructionScript)

(fn SphereLimited
  (params (Sphere :type Scene%20Component%20Object%20Reference))
  (Transformation|SetWorldRotation Sphere (Math|Rotator|MakeRotator 0.0 (Math|Float|Clamp(Float) (.pitch (Transformation|GetWorldRotation Sphere)) -9e+01 9e+01) 0.0) false false))